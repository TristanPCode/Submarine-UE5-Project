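; BP_SubmarineSpectator is the spectator for the submarine game, acting as the input layer for spectator movement and camera control.
; Input action events for directional keys (left, right, up, down) and the third-person camera toggle forward presses and releases to matching Spectator functions.
; Mouse X/Y and scroll zoom pass their values through the same way.
; The handlers are defined outside this graph, which holds no logic of its own.
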(event `EnhancedInput|/Game/Input/InputAction_SpectatorRight`
  (params (ActionValue :type "Float (double-precision)") (ElapsedSeconds :type "Float (double-precision)") (TriggeredSeconds :type "Float (double-precision)") (InputAction :type "InputAction Object Reference" :default "/Game/Input/InputAction_SpectatorRight.InputAction_SpectatorRight"))
  (:`Started`
    (`self.SpectatorRightPressed`))
  (:`Completed`
    (`self.SpectatorRightReleased`)))

(event `EnhancedInput|/Game/Input/InputAction_MouseX`
  (params (ActionValue :type "Float (double-precision)") (ElapsedSeconds :type "Float (double-precision)") (TriggeredSeconds :type "Float (double-precision)") (InputAction :type "InputAction Object Reference" :default "/Game/Input/InputAction_MouseX.InputAction_MouseX"))
  (:`Triggered`
    (`self.SpectatorMouseX` ActionValue)))

(event `EnhancedInput|/Game/Input/InputAction_SpectatorLeft`
  (params (ActionValue :type "Float (double-precision)") (ElapsedSeconds :type "Float (double-precision)") (TriggeredSeconds :type "Float (double-precision)") (InputAction :type "InputAction Object Reference" :default "/Game/Input/InputAction_SpectatorLeft.InputAction_SpectatorLeft"))
  (:`Started`
    (`self.SpectatorLeftPressed`))
  (:`Completed`
    (`self.SpectatorLeftReleased`)))

(event `EnhancedInput|/Game/Input/InputAction_MouseY`
  (params (ActionValue :type "Float (double-precision)") (ElapsedSeconds :type "Float (double-precision)") (TriggeredSeconds :type "Float (double-precision)") (InputAction :type "InputAction Object Reference" :default "/Game/Input/InputAction_MouseY.InputAction_MouseY"))
  (:`Triggered`
    (`self.SpectatorMouseY` ActionValue)))

(event `EnhancedInput|/Game/Input/InputAction_ScrollZoom`
  (params (ActionValue :type "Float (double-precision)") (ElapsedSeconds :type "Float (double-precision)") (TriggeredSeconds :type "Float (double-precision)") (InputAction :type "InputAction Object Reference" :default "/Game/Input/InputAction_ScrollZoom.InputAction_ScrollZoom"))
  (:`Triggered`
    (`self.SpectatorScrollZoom` ActionValue)))

(event `EnhancedInput|/Game/Input/InputAction_SpectatorUp`
  (params (ActionValue :type "Float (double-precision)") (ElapsedSeconds :type "Float (double-precision)") (TriggeredSeconds :type "Float (double-precision)") (InputAction :type "InputAction Object Reference" :default "/Game/Input/InputAction_SpectatorUp.InputAction_SpectatorUp"))
  (:`Started`
    (`self.SpectatorUpPressed`))
  (:`Completed`
    (`self.SpectatorUpReleased`)))

(event `EnhancedInput|/Game/Input/InputAction_Camera3rdView`
  (params (ActionValue :type "Float (double-precision)") (ElapsedSeconds :type "Float (double-precision)") (TriggeredSeconds :type "Float (double-precision)") (InputAction :type "InputAction Object Reference" :default "/Game/Input/InputAction_Camera3rdView.InputAction_Camera3rdView"))
  (:`Started`
    (`self.SpectatorCameraTogglePressed`))
  (:`Completed`
    (`self.SpectatorCameraToggleReleased`)))

(event `EnhancedInput|/Game/Input/InputAction_SpectatorDown`
  (params (ActionValue :type "Float (double-precision)") (ElapsedSeconds :type "Float (double-precision)") (TriggeredSeconds :type "Float (double-precision)") (InputAction :type "InputAction Object Reference" :default "/Game/Input/InputAction_SpectatorDown.InputAction_SpectatorDown"))
  (:`Started`
    (`self.SpectatorDownPressed`))
  (:`Completed`
    (`self.SpectatorDownReleased`)))

(fn `UserConstructionScript`)